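; Farm tile actor that grows wheat, corn or pumpkin from the player's selected seed and releases loose crop pickups when harvested.
; PlantSeed uses up a seed from the character and starts that crop's chain, swapping seed and growth-phase meshes between one-second Delay-loop countdowns shown on Timer text.
; A random disease roll after each countdown can halt growth with a diseased material.
; Activate calls Harvest, which clears the tile; diseased plants yield nothing.
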(event `PlantWheat`
  (bind _returnvalue (`AddComponent|NODE_AddStaticMeshComponent-0` :`RelativeTransform` (`KismetMathLibrary.MakeTransform` (`self.Relative Transform Location_Seed`))))
  (`self.GrowTime` (`self.WheatGrowTime`)
    (:`Out`
      (`self.Chance of Disease` _returnvalue
        (:`Output`
          (`ActorComponent.K2_DestroyComponent` _returnvalue)
          (bind _returnvalue_2 (`AddComponent|NODE_AddStaticMeshComponent-1` :`RelativeTransform` (`KismetMathLibrary.MakeTransform` (`self.Relative Transform Location_Phase1`))))
          (`self.GrowTime` (`self.WheatGrowTime`)
            (:`Out`
              (`self.Chance of Disease` _returnvalue_2
                (:`Output`
                  (`ActorComponent.K2_DestroyComponent` _returnvalue_2)
                  (bind _returnvalue_3 (`AddComponent|NODE_AddStaticMeshComponent-2` :`RelativeTransform` (`KismetMathLibrary.MakeTransform` (`self.Relative Transform Location_Phase2`))))
                  (set `self.FullyGrown?` true)
                  (set `self.CurrentMesh` _returnvalue_3)
                  (set `self.WhatCanBeHarvested?` "Wheat"))))))))))

(event `PlantCorn`
  (bind _returnvalue (`AddComponent|NODE_AddStaticMeshComponent-6` :`RelativeTransform` (`KismetMathLibrary.MakeTransform` (`self.Relative Transform Location_Seed`))))
  (`self.GrowTime` (`self.CornGrowTime`)
    (:`Out`
      (`self.Chance of Disease` _returnvalue
        (:`Output`
          (`ActorComponent.K2_DestroyComponent` _returnvalue)
          (bind _returnvalue_2 (`AddComponent|NODE_AddStaticMeshComponent-7` :`RelativeTransform` (`KismetMathLibrary.MakeTransform` (`self.Relative Transform Location_Phase1`))))
          (`self.GrowTime` (`self.CornGrowTime`)
            (:`Out`
              (`self.Chance of Disease` _returnvalue_2
                (:`Output`
                  (`ActorComponent.K2_DestroyComponent` _returnvalue_2)
                  (bind _returnvalue_3 (`AddComponent|NODE_AddStaticMeshComponent-8` :`RelativeTransform` (`KismetMathLibrary.MakeTransform` (`self.Relative Transform Location_Phase2`))))
                  (set `self.FullyGrown?` true)
                  (set `self.CurrentMesh` _returnvalue_3)
                  (set `self.WhatCanBeHarvested?` "Corn"))))))))))

(event `PlantPumpkin`
  (bind _returnvalue (`AddComponent|NODE_AddStaticMeshComponent-3` :`RelativeTransform` (`KismetMathLibrary.MakeTransform` (`self.Relative Transform Location_Seed`))))
  (`self.GrowTime` (`self.PumpkinGrowTime`)
    (:`Out`
      (`self.Chance of Disease` _returnvalue
        (:`Output`
          (`ActorComponent.K2_DestroyComponent` _returnvalue)
          (bind _returnvalue_2 (`AddComponent|NODE_AddStaticMeshComponent-4` :`RelativeTransform` (`KismetMathLibrary.MakeTransform` (`self.Relative Transform Location_Phase1`))))
          (`self.GrowTime` (`self.PumpkinGrowTime`)
            (:`Out`
              (`self.Chance of Disease` _returnvalue_2
                (:`Output`
                  (`ActorComponent.K2_DestroyComponent` _returnvalue_2)
                  (bind _returnvalue_3 (`AddComponent|NODE_AddStaticMeshComponent-5` :`RelativeTransform` (`KismetMathLibrary.MakeTransform` (`self.Relative Transform Location_Phase2`))))
                  (set `self.FullyGrown?` true)
                  (set `self.CurrentMesh` _returnvalue_3)
                  (set `self.WhatCanBeHarvested?` "Pumpkin"))))))))))

(event `/Game/Blueprints/Harvest/BPI_Activate.Activate`
  (`self.Harvest`))

(event `/Game/Blueprints/Harvest/BPI_PlantSeed.PlantSeed`
  (if (not (`self.isSomethingPlanted`))
    (bind _asbp_third_person_character (cast `/Game/ThirdPerson/Blueprints/BP_ThirdPersonCharacter` (`GameplayStatics.GetPlayerCharacter` 0)))
    (switch `int` (`/Game/ThirdPerson/Blueprints/BP_ThirdPersonCharacter.Seed` _asbp_third_person_character)
      (:`0`
        (`self.DoWeHaveWheatSeeds`
          (:`Output`
            (`self.PlantWheat`))))
      (:`1`
        (`self.DoWeHaveCornSeeds`
          (:`Output`
            (`self.PlantCorn`))))
      (:`2`
        (`self.DoWeHavePumpkinSeeds`
          (:`Output`
            (`self.PlantPumpkin`)))))
    (set `self.isSomethingPlanted` true)))

(event `self.ReceiveBeginPlay`
  (set `Text3DComponent.Text` (`self.Value`) (`self.Timer`)))

(fn `Harvest`
  (bind _returnvalue (`KismetMathLibrary.Conv_VectorToTransform` (`SceneComponent.K2_GetComponentLocation` (`self.Timer`))))
  (if (`self.FullyGrown?`)
    (`ActorComponent.K2_DestroyComponent` (`self.CurrentMesh`))
    (switch `string` (`self.WhatCanBeHarvested?`)
      (:`Default`
        _)
      (:`Wheat`
        (`|SpawnActorFromClass` "/Game/Blueprints/Harvest/BP_Wheat_Loose.BP_Wheat_Loose_C" _returnvalue "Undefined" "MultiplyWithRoot" null null))
      (:`Corn`
        (`|SpawnActorFromClass` "/Game/Blueprints/Harvest/BP_Corn_Loose.BP_Corn_Loose_C" _returnvalue "Undefined" "MultiplyWithRoot" null null))
      (:`Pumpkin`
        (`|SpawnActorFromClass` "/Game/Blueprints/Harvest/BP_Pumpkin_Loose.BP_Pumpkin_Loose_C" _returnvalue "Undefined" "MultiplyWithRoot" null null)))
    (set `self.FullyGrown?` false)
    (set `self.CurrentMesh` null)
    (set `self.isSomethingPlanted` false)
    (set `self.WhatCanBeHarvested?` "")))

(fn `UserConstructionScript`)