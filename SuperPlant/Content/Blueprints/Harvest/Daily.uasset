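; Daily harvest Blueprint that relays a PlantMoney event to the player character.
; PlantMoney casts player 0's character to BP_ThirdPersonCharacter and calls TriggerDaily, so the resulting behavior lives in that character.
; The remaining graph is unreachable leftover logic that steps Entertainment, Super, Emergency and Expenses budget buckets up or down through chained increments and decrements, printing each result.
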(event `self.ReceiveBeginPlay`)

(event `/Game/Blueprints/Harvest/BPI_PlantMoney.PlantMoney`
  (bind _asbp_third_person_character (cast `/Game/ThirdPerson/Blueprints/BP_ThirdPersonCharacter` (`GameplayStatics.GetPlayerCharacter` 0)))
  (`/Game/ThirdPerson/Blueprints/BP_ThirdPersonCharacter.TriggerDaily` _asbp_third_person_character))

(fn `UserConstructionScript`)