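; SuperAccount is a harvest-game actor that responds to planting money in what appears to be the super savings bucket.
; PlantMoney calls Stage6 and TriggerSuper on the player's third-person character, then spawns a Coin at its Sphere.
; A debug print follows the spawn, and a coin-drop sound plays there after a short delay.
; Disconnected leftover chains that step Entertainment, Super, Emergency and Expenses bucket values up or down never run.
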(event `self.PlantMoney`
  (bind _returnvalue (`SceneComponent.K2_GetComponentLocation` (`self.Sphere`)))
  (bind _asbp_third_person_character (cast `/Game/ThirdPerson/Blueprints/BP_ThirdPersonCharacter` (`GameplayStatics.GetPlayerCharacter` 0)))
  (`/Game/ThirdPerson/Blueprints/BP_ThirdPersonCharacter.Stage 6` _asbp_third_person_character)
  (`/Game/ThirdPerson/Blueprints/BP_ThirdPersonCharacter.Trigger Super` _asbp_third_person_character)
  (`|SpawnActorFromClass` "/Game/Blueprints/Harvest/Coin.Coin_C" (`KismetMathLibrary.Conv_VectorToTransform` _returnvalue) "AlwaysSpawn" "MultiplyWithRoot" null null)
  (`KismetSystemLibrary.PrintString` "COIN SPAWNED")
  (`KismetSystemLibrary.Delay` 0.7)
  (`GameplayStatics.PlaySoundAtLocation` "/Game/Blueprints/Harvest/coins-dropped-ni-sound-1-1-00-00__1_.coins-dropped-ni-sound-1-1-00-00__1_" _returnvalue (struct) 1.0 1.0 0.0 null null null null))

(fn `UserConstructionScript`)