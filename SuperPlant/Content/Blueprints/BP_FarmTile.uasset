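; BP_FarmTile is a farm plot Blueprint that plants and grows a crop based on the player character's selected seed, with wheat the only crop handled.
; PlantSeed accepts one planting on an empty tile, then PlantWheat swaps through three static mesh stages, separated by timed waits.
; The GrowTime macro loops a one-second Delay to drive a countdown text.
; The final stage stores its mesh and flags the tile as harvestable wheat.
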(event `self.ReceiveBeginPlay`
  (set `Text3DComponent.Text` (`self.Value`) (`self.Timer`)))

(event `/Game/Blueprints/BPI_PlantSeed.PlantSeed`
  (if (not (`self.isSomethingPlanted`))
    (bind _asbp_third_person_character (cast `/Game/ThirdPerson/Blueprints/BP_ThirdPersonCharacter` (`GameplayStatics.GetPlayerCharacter` 0)))
    (switch `int` (`/Game/ThirdPerson/Blueprints/BP_ThirdPersonCharacter.Seed` _asbp_third_person_character)
      (:`0`
        (`self.PlantWheat`)
        (set `self.isSomethingPlanted` true)))))

(event `PlantWheat`
  (bind _relativetranformlocation (`self.RelativeTranformLocation`))
  (bind _returnvalue (`AddComponent|NODE_AddStaticMeshComponent-0` :`RelativeTransform` (`KismetMathLibrary.MakeTransform` _relativetranformlocation)))
  (`self.GrowTime` (`self.WheatGrowTime`)
    (:`Out`
      (`ActorComponent.K2_DestroyComponent` _returnvalue)
      (bind _returnvalue_2 (`AddComponent|NODE_AddStaticMeshComponent-1` :`RelativeTransform` (`KismetMathLibrary.MakeTransform` _relativetranformlocation)))
      (`self.GrowTime` (`self.WheatGrowTime`)
        (:`Out`
          (`ActorComponent.K2_DestroyComponent` _returnvalue_2)
          (bind _returnvalue_3 (`AddComponent|NODE_AddStaticMeshComponent-2` :`RelativeTransform` (`KismetMathLibrary.MakeTransform` _relativetranformlocation)))
          (set `self.FullyGrown?` true)
          (set `self.CurrentMesh` _returnvalue_3)
          (set `self.WhatCanBeHarvested?` "Wheat"))))))

(fn `UserConstructionScript`)