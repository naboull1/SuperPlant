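; BP_TreeEmergency is a tree branch actor, apparently for an emergency savings bucket, built procedurally from spline meshes.
; The construction script requires a valid BucketUI reference, which is only created on BeginPlay, and immediately overwrites its EmergencyBckt value.
; Segment count derives from branch length, clamped; direction values bend the spline, and one mesh spans each point pair.
; Old-mesh destruction, fixed-segment and investment-scaling logic are disconnected.
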(event `self.ReceiveBeginPlay`
  (bind _returnvalue (`|CreateWidget` "/Game/UI/BucketUI.BucketUI_C"))
  (set `self.Widget Ref` _returnvalue))

(fn `UserConstructionScript`
  (bind _spline (`self.Spline`))
  (bind _spline_2 (`self.Spline`))
  (bind _asbucket_ui (cast `/Game/UI/BucketUI` (`self.Widget Ref`)))
  (set `self.BranchEmergencyPoints` (`/Game/UI/BucketUI.Emergency Bckt` _asbucket_ui))
  (for _array_element (`self.GeneratedSplineMeshes`)
    _)
  (`KismetArrayLibrary.Array_Clear` (`self.GeneratedSplineMeshes`))
  (set `self.BranchEmergencyPoints` (`KismetMathLibrary.Clamp` (`KismetMathLibrary.FFloor` (/ (`self.BranchSuperLength`) (`self.SegmentLength`))) 1 (`self.MaxSegments`)))
  (`SplineComponent.ClearSplinePoints` _spline true)
  (for _index (range (+ (`self.BranchEmergencyPoints`) 1))
    (bind _returnvalue (`KismetMathLibrary.Conv_IntToDouble` _index))
    (`SplineComponent.AddSplinePoint` _spline (`KismetMathLibrary.MakeVector` (`KismetMathLibrary.FClamp` (* _returnvalue (`self.BranchSuper_DirectionX`)) -60.0 60.0) (`KismetMathLibrary.FClamp` (* _returnvalue (`self.BranchSuper_DirectionY`)) -40.0 40.0) (* _returnvalue (`self.SegmentLength`))) "Local" true))
  (for _index_2 (range (`self.BranchEmergencyPoints`))
    (bind _returnvalue_2 (`AddComponent|NODE_AddSplineMeshComponent-0`))
    (`StaticMeshComponent.SetStaticMesh` _returnvalue_2 (`self.branchSegmenMesh`))
    (`SplineMeshComponent.SetForwardAxis` _returnvalue_2 "Y" true)
    (`KismetArrayLibrary.Array_Add` (`self.GeneratedSplineMeshes`) _returnvalue_2)
    (bind _returnvalue_3 (+ _index_2 1))
    (`SplineMeshComponent.SetStartAndEnd` _returnvalue_2 (`SplineComponent.GetLocationAtSplinePoint` _spline_2 _index_2 "Local") (`SplineComponent.GetTangentAtSplinePoint` _spline_2 _index_2 "Local") (`SplineComponent.GetLocationAtSplinePoint` _spline_2 _returnvalue_3 "Local") (`SplineComponent.GetTangentAtSplinePoint` _spline_2 _returnvalue_3 "Local") true)))