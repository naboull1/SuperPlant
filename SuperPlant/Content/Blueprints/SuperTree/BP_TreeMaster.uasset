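; BP_TreeMaster is a tree actor that procedurally builds its "Super" branch in the Construction Script, with no runtime logic.
; Branch length over segment length sets a clamped segment count, and spline points climb in Z with clamped X/Y lean.
; Five fixed spline meshes follow successive points, shown according to that count.
; Disconnected nodes hold unused bend adjustments and Z scaling for investment-category branches.
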(fn `UserConstructionScript`
  (bind _spline (`self.Spline`))
  (bind _spline_2 (`self.Spline`))
  (bind _spline_3 (`self.Spline`))
  (bind _spline_4 (`self.Spline`))
  (bind _spline_5 (`self.Spline`))
  (bind _spline_6 (`self.Spline`))
  (bind _spline_7 (`self.Spline`))
  (set `self.BranchSuperPoints` (`KismetMathLibrary.Clamp` (`KismetMathLibrary.FFloor` (/ (`self.BranchSuperLength`) (`self.SegmentLength`))) 1 (`self.MaxSegments`)))
  (`SplineComponent.ClearSplinePoints` _spline_2 true)
  (for _index (range (+ (`self.BranchSuperPoints`) 1))
    (bind _returnvalue (`KismetMathLibrary.Conv_IntToDouble` _index))
    (`SplineComponent.AddSplinePoint` _spline_2 (`KismetMathLibrary.MakeVector` (`KismetMathLibrary.FClamp` (* _returnvalue (`self.BranchSuper_DirectionX`)) -60.0 60.0) (`KismetMathLibrary.FClamp` (* _returnvalue (`self.BranchSuper_DirectionY`)) -40.0 40.0) (* _returnvalue (`self.SegmentLength`))) "Local" true)
    (`SplineMeshComponent.SetStartAndEnd` (`self.SplineMesh`) (`SplineComponent.GetLocationAtSplinePoint` _spline_3 0 "Local") (`SplineComponent.GetTangentAtSplinePoint` _spline_3 0 "Local") (`SplineComponent.GetLocationAtSplinePoint` _spline_3 1 "Local") (`SplineComponent.GetTangentAtSplinePoint` _spline_3 1 "Local") true)
    (`SceneComponent.SetVisibility` (`self.SplineMesh`) (>= (`self.BranchSuperPoints`) 1) false)
    (`SplineMeshComponent.SetStartAndEnd` (`self.SplineMesh_2`) (`SplineComponent.GetLocationAtSplinePoint` _spline_4 1 "Local") (`SplineComponent.GetTangentAtSplinePoint` _spline_4 1 "Local") (`SplineComponent.GetLocationAtSplinePoint` _spline_4 2 "Local") (`SplineComponent.GetTangentAtSplinePoint` _spline_4 2 "Local") true)
    (`SceneComponent.SetVisibility` (`self.SplineMesh_2`) (>= (`self.BranchSuperPoints`) 2) false)
    (`SplineMeshComponent.SetStartAndEnd` (`self.SplineMesh_3`) (`SplineComponent.GetLocationAtSplinePoint` _spline_5 2 "Local") (`SplineComponent.GetTangentAtSplinePoint` _spline_5 2 "Local") (`SplineComponent.GetLocationAtSplinePoint` _spline_5 3 "Local") (`SplineComponent.GetTangentAtSplinePoint` _spline_5 3 "Local") true)
    (`SceneComponent.SetVisibility` (`self.SplineMesh_3`) (>= (`self.BranchSuperPoints`) 3) false)
    (`SplineMeshComponent.SetStartAndEnd` (`self.SplineMesh_4`) (`SplineComponent.GetLocationAtSplinePoint` _spline_6 3 "Local") (`SplineComponent.GetTangentAtSplinePoint` _spline_6 3 "Local") (`SplineComponent.GetLocationAtSplinePoint` _spline_6 4 "Local") (`SplineComponent.GetTangentAtSplinePoint` _spline_6 4 "Local") true)
    (`SceneComponent.SetVisibility` (`self.SplineMesh_4`) (>= (`self.BranchSuperPoints`) 4) false)
    (`SplineMeshComponent.SetStartAndEnd` (`self.SplineMesh_4`) (`SplineComponent.GetLocationAtSplinePoint` _spline_7 3 "Local") (`SplineComponent.GetTangentAtSplinePoint` _spline_7 3 "Local") (`SplineComponent.GetLocationAtSplinePoint` _spline_7 4 "Local") (`SplineComponent.GetTangentAtSplinePoint` _spline_7 4 "Local") true)
    (`SceneComponent.SetVisibility` (`self.SplineMesh_5`) (>= (`self.BranchSuperPoints`) 5) false)
    (`SplineMeshComponent.SetStartAndEnd` (`self.SplineMesh_5`) (`SplineComponent.GetLocationAtSplinePoint` _spline 4 "Local") (`SplineComponent.GetTangentAtSplinePoint` _spline 4 "Local") (`SplineComponent.GetLocationAtSplinePoint` _spline 5 "Local") (`SplineComponent.GetTangentAtSplinePoint` _spline 5 "Local") true)))