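; Guide-line actor that draws an animated navigation path from its location toward a Destination using spline meshes.
; Unless Editable is set, the construction script rebuilds the spline with evenly spaced points along a straight line at the given Interval.
; Each segment becomes a spline mesh with a dynamic material for speed, color and twinkle.
; Segments use overlap collision and can hide individually when overlapped, if EnableOverlappedDisappear is on.
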(event `self.ReceiveTick`
  (params (DeltaSeconds :type "Float (single-precision)")))

(fn `BP_Navigation_AutoGenFunc`
  (params (OverlappedComponent :type "PrimitiveComponent Object Reference") (OtherActor :type "Actor Object Reference") (OtherComp :type "PrimitiveComponent Object Reference") (OtherBodyIndex :type Integer) (bFromSweep :type Boolean) (SweepResult :type "HitResult Structure (by ref)"))
  ;[1 1 1] Interactive logic
  (if (`self.EnableOverlappedDisappear`)
    (`SceneComponent.SetVisibility` OverlappedComponent false false)
    (return)))

(fn `CalMiddlePoint`
  (params (DestPoint :type "Vector Structure") (StartPoint :type "Vector Structure") (Index :type Integer))
  (returns (MiddlePoint :type "Vector Structure"))
  (bind _returnvalue (`KismetMathLibrary.Conv_IntToDouble` Index))
  (bind _x (.x StartPoint))
  (bind _y (.y StartPoint))
  (bind _z (.z StartPoint))
  (return (`KismetMathLibrary.MakeVector` (+ (* (* (/ (- (.x DestPoint) _x) (`self.Distance`)) _returnvalue) (`self.interval`)) _x) (+ (* (* (/ (- (.y DestPoint) _y) (`self.Distance`)) _returnvalue) (`self.interval`)) _y) (+ (* (* (/ (- (.z DestPoint) _z) (`self.Distance`)) _returnvalue) (`self.interval`)) _z))))

(fn `UserConstructionScript`
  (bind _returnvalue (`self.K2_GetActorLocation`))
  (bind _spline (`self.Spline`))
  (if (not (`self.Editable`))
    ;[1 1 1] Calculate the number of intermediate points
    (`SplineComponent.ClearSplinePoints` (`self.Spline`) true)
    (set `self.StartingPoint` _returnvalue)
    (set `self.Distance` (`KismetMathLibrary.Vector_Distance` (`self.Destination`) _returnvalue))
    (for _index (range (+ (`KismetMathLibrary.FTrunc` (/ (`self.Distance`) (`self.interval`))) 1))
      (bind _middlepoint (`self.CalMiddlePoint` (`self.Destination`) (`self.StartingPoint`) _index))
      (bind _output_get (set `self.Temp` _middlepoint))
      (`SplineComponent.AddSplinePoint` (`self.Spline`) _output_get "World" true)))
  (for _index_2 (range (+ (- (`SplineComponent.GetNumberOfSplinePoints` (`self.Spline`)) 2) 1))
    (bind _returnvalue_2 (`AddComponent|NODE_AddSplineMeshComponent-0`))
    (add `PrimitiveComponent.OnComponentBeginOverlap` _returnvalue_2 (`|CreateDelegate` :!event `BP_Navigation_AutoGenFunc`))
    (`StaticMeshComponent.SetStaticMesh` _returnvalue_2 (`self.UnitMesh`))
    (`SplineMeshComponent.SetForwardAxis` _returnvalue_2 (`self.forwardAxis`) true)
    ;[1 1 1] Set appearance
    (bind _returnvalue_3 (`PrimitiveComponent.CreateDynamicMaterialInstance` _returnvalue_2 0 (`self.Material`) "None"))
    (`MaterialInstanceDynamic.SetScalarParameterValue` _returnvalue_3 "Speed" (`self.Speed`))
    (`MaterialInstanceDynamic.SetVectorParameterValue` _returnvalue_3 "Color" (`self.Color`))
    (`MaterialInstanceDynamic.SetScalarParameterValue` _returnvalue_3 "twinkle" (`self.twinkle`))
    (`PrimitiveComponent.SetMaterial` _returnvalue_2 0 _returnvalue_3)
    ;[1 1 1] Build path
    (`SceneComponent.K2_AttachToComponent` _returnvalue_2 (`self.Spline`) "None" "KeepRelative" "KeepRelative" "KeepRelative" true)
    (bind _returnvalue_4 (+ _index_2 1))
    (`SplineMeshComponent.SetStartAndEnd` _returnvalue_2 (`SplineComponent.GetLocationAtSplinePoint` _spline _index_2 "Local") (`SplineComponent.GetTangentAtSplinePoint` _spline _index_2 "Local") (`SplineComponent.GetLocationAtSplinePoint` _spline _returnvalue_4 "Local") (`SplineComponent.GetTangentAtSplinePoint` _spline _returnvalue_4 "Local") true)
    (`PrimitiveComponent.SetCollisionResponseToAllChannels` _returnvalue_2 "ECR_Overlap")
    (`PrimitiveComponent.SetCollisionEnabled` _returnvalue_2 "QueryAndPhysics")
    (`PrimitiveComponent.SetCollisionObjectType` _returnvalue_2 "ECC_WorldDynamic")))