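; BP_Navigation is a spline-based guide line that draws a visual path in the level.
; The construction script adds a spline mesh per segment, matched to point positions and tangents, with a dynamic material driven by speed, color and twinkle parameters.
; Segments overlap all channels and bind an overlap handler that, when EnableOverlappedDisappear is set, hides the touched segment, whatever actor touches it.
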(fn `BP_Navigation_AutoGenFunc`
  (params (OverlappedComponent :type "PrimitiveComponent Object Reference") (OtherActor :type "Actor Object Reference") (OtherComp :type "PrimitiveComponent Object Reference") (OtherBodyIndex :type Integer) (bFromSweep :type Boolean) (SweepResult :type "HitResult Structure (by ref)"))
  ;[1 1 1] Interactive logic
  (if (`self.EnableOverlappedDisappear`)
    (`SceneComponent.SetVisibility` OverlappedComponent false false)
    (return)))

(fn `UserConstructionScript`
  (bind _spline (`self.Spline`))
  (for _index (range (+ (- (`SplineComponent.GetNumberOfSplinePoints` (`self.Spline`)) 2) 1))
    (bind _returnvalue (`AddComponent|NODE_AddSplineMeshComponent-0`))
    (add `PrimitiveComponent.OnComponentBeginOverlap` _returnvalue (`|CreateDelegate` :!event `BP_Navigation_AutoGenFunc`))
    (`StaticMeshComponent.SetStaticMesh` _returnvalue (`self.UnitMesh`))
    (`SplineMeshComponent.SetForwardAxis` _returnvalue (`self.forwardAxis`) true)
    ;[1 1 1] Set appearance
    (bind _returnvalue_2 (`PrimitiveComponent.CreateDynamicMaterialInstance` _returnvalue 0 (`self.Material`) "None"))
    (`MaterialInstanceDynamic.SetScalarParameterValue` _returnvalue_2 "Speed" (`self.Speed`))
    (`MaterialInstanceDynamic.SetVectorParameterValue` _returnvalue_2 "Color" (`self.Color`))
    (`MaterialInstanceDynamic.SetScalarParameterValue` _returnvalue_2 "twinkle" (`self.twinkle`))
    (`PrimitiveComponent.SetMaterial` _returnvalue 0 _returnvalue_2)
    ;[1 1 1] Build path
    (`SceneComponent.K2_AttachToComponent` _returnvalue (`self.Spline`) "None" "KeepRelative" "KeepRelative" "KeepRelative" true)
    (bind _returnvalue_3 (+ _index 1))
    (`SplineMeshComponent.SetStartAndEnd` _returnvalue (`SplineComponent.GetLocationAtSplinePoint` _spline _index "Local") (`SplineComponent.GetTangentAtSplinePoint` _spline _index "Local") (`SplineComponent.GetLocationAtSplinePoint` _spline _returnvalue_3 "Local") (`SplineComponent.GetTangentAtSplinePoint` _spline _returnvalue_3 "Local") true)
    (`PrimitiveComponent.SetCollisionResponseToAllChannels` _returnvalue "ECR_Overlap")
    (`PrimitiveComponent.SetCollisionEnabled` _returnvalue "QueryAndPhysics")
    (`PrimitiveComponent.SetCollisionObjectType` _returnvalue "ECC_WorldDynamic")))